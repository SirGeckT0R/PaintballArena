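; Projectile weapon Blueprint whose graphs hold only debug visualization, with no firing or projectile logic.
; Every tick it draws a debug arrow from the muzzle component along its forward vector to show the aim direction.
; An unconnected print of the AmmoManager's magazine and total ammo counts never runs, and the construction script is empty.
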(event `self.ReceiveTick`
  (params (DeltaSeconds :type "Float (single-precision)"))
  (bind _muzzlecomponent (`self.MuzzleComponent`))
  (bind _returnvalue (`SceneComponent.K2_GetComponentLocation` _muzzlecomponent))
  (`KismetSystemLibrary.DrawDebugArrow` _returnvalue (+ _returnvalue (* (`SceneComponent.GetForwardVector` _muzzlecomponent) 4000.0)) 2.0 (struct :`R` 1.0 :`G` 0.06108 :`A` 1.0) 1.0 2.0))

(fn `UserConstructionScript`)