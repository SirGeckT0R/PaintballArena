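; Base enemy character that takes damage, reacts to hits, carries a weapon and drops an ammo pickup on death.
; Health logic is delegated to a damage system component, whose death and damage-response events are bound in the construction script.
; Hits freeze the AI controller during a reaction montage, then switch it to attacking the damage causer or dead.
; Tick turns the health bar widget toward the player camera and polls for death.
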(event `self.ReceiveTick`
  (params (DeltaSeconds :type "Float (single-precision)"))
  (`self.RotateHealthBarToPlayer`)
  (bind _isdead (`self.IsDead`))
  (if _isdead
    (`AIEnemyBase.SetStateAsDead` (`self.AICEnemyBase`))))

(event `self.ReceiveBeginPlay`
  (`KismetSystemLibrary.Delay` 0.2)
  (bind _asaic_new_enemy_base (cast `/Game/Blueprints/Enemies/AI/AIC_NewEnemyBase` (`AIBlueprintHelperLibrary.GetAIController` self)))
  (set `self.AICEnemyBase` _asaic_new_enemy_base)
  (bind _aswb_health_bar (cast `/Game/Blueprints/UI/WB_HealthBar` (`WidgetComponent.GetWidget` (`self.HealthBarWidget`))))
  (set `self.HealthBar` _aswb_health_bar)
  (`self.UpdateHealthBar`))

(event `self.ReceiveAnyDamage`
  (params (Damage :type "Float (single-precision)") (DamageType :type "DamageType Object Reference") (InstigatedBy :type "Controller Object Reference") (DamageCauser :type "Actor Object Reference"))
  (`self.TakeDamage` (make `/Game/Blueprints/DamageSystem/S_DamageInfo` Damage "NewEnumerator2") DamageCauser)
  (`self.UpdateHealthBar`))

(event `Death`
  (`ActorComponent.K2_DestroyComponent` (`self.HealthBarWidget`))
  (`EnemyAI.UnequipWeapon`)
  (`self.OnWeaponUnequipped`)
  (`|SpawnActorFromClass` "/Game/Blueprints/Weapons/BP_AmmoPickup.BP_AmmoPickup_C" (`self.GetTransform`) "AlwaysSpawn" "MultiplyWithRoot" null null)
  (`KismetSystemLibrary.Delay` 0.1)
  (`AIEnemyBase.SetStateAsDead` (`self.AICEnemyBase`)))

(event `HitResponse`
  (params (DamageResponse :type "/Game/Blueprints/DamageSystem/E_DamageResponse Enum" :default "NewEnumerator0") (DamageCauser :type "Actor Object Reference"))
  (bind _aicenemybase (`self.AICEnemyBase`))
  (`MovementComponent.StopMovementImmediately` (`self.CharacterMovement`))
  (`/Game/Blueprints/Enemies/AI/AIC_EnemyBase.SetStateAsFrozen` (`.AICEnemyBase` (`self.AICEnemyBase`)))
  (`|PlayMontage` (`self.Mesh`) (`self.HitReactionMontage`)
    (:`OnCompleted`
      _)
    (:`OnInterrupted`
      _))
  (bind _isdead (`self.IsDead`))
  (if _isdead
    (`AIEnemyBase.SetStateAsDead` _aicenemybase)
    (else
      (`AIEnemyBase.SetStateAsAttacking` _aicenemybase DamageCauser true)
      (`/Game/Blueprints/Enemies/AI/AIC_EnemyBase.OnHostileDetected` DamageCauser))))

(event `self.EquipWeapon`
  (`self.SpawnWeapon` (struct))
  (`self.K2_AttachToComponent` (`self.Weapon`) (`self.Mesh`) "RightHandWeaponSocket" "KeepRelative" "KeepRelative" "KeepRelative" true)
  (`self.OnWeaponEquipped`))

(event `self.UnequipWeapon`
  (bind _weapon (`self.Weapon`))
  (`self.K2_DetachFromActor` _weapon "KeepRelative" "KeepRelative" "KeepRelative")
  (`self.K2_DestroyActor` _weapon))

(fn `GetCurrentHealth`
  (returns (CurrentHealth :type "Float (double-precision)"))
  (return (`/Game/Blueprints/DamageSystem/BPC_DamageSystem.Health` (`self.BPC_DamageSystem`))))

(fn `GetMaxHealth`
  (returns (MaxHealth :type "Float (double-precision)"))
  (return (`/Game/Blueprints/DamageSystem/BPC_DamageSystem.MaxHealth` (`self.BPC_DamageSystem`))))

(fn `Heal`
  (params (Amount :type "Float (double-precision)"))
  (returns (NewHealth :type "Float (double-precision)"))
  (`/Game/Blueprints/DamageSystem/BPC_DamageSystem.Heal` (`self.BPC_DamageSystem`) 0.0)
  (`self.UpdateHealthBar`)
  (return 0.0))

(fn `IsDead`
  (returns (IsDead :type Boolean))
  (return (`/Game/Blueprints/DamageSystem/BPC_DamageSystem.IsDead` (`self.BPC_DamageSystem`))))

(fn `RotateHealthBarToPlayer`
  (bind _healthbarwidget (`self.HealthBarWidget`))
  (`/Engine/EditorBlueprintResources/StandardMacros.IsValid` (`self.HealthBarWidget`)
    (:`Is Valid`
      (`SceneComponent.K2_SetWorldRotation` _healthbarwidget (`KismetMathLibrary.ComposeRotators` (`KismetMathLibrary.FindLookAtRotation` (`PlayerCameraManager.GetCameraLocation` (`GameplayStatics.GetPlayerCameraManager` 0)) (`SceneComponent.K2_GetComponentLocation` _healthbarwidget)) (struct :`Yaw` 180.0)) false false))))

(fn `TakeDamage`
  (params (DamageInfo :type "/Game/Blueprints/DamageSystem/S_DamageInfo Structure") (`DamageCauser ` :type "Actor Object Reference"))
  (returns (WasDamaged :type Boolean))
  (bind _wasdamaged (`/Game/Blueprints/DamageSystem/BPC_DamageSystem.TakeDamage` (`self.BPC_DamageSystem`) DamageInfo `DamageCauser `))
  (`self.UpdateHealthBar`)
  (return _wasdamaged))

(fn `UpdateHealthBar`
  (bind _currenthealth (`self.GetCurrentHealth`))
  (`/Game/Blueprints/UI/WB_HealthBar.SetHealth` (`self.HealthBar`) _currenthealth)
  (return))

(fn `UserConstructionScript`
  (bind _bpc_damagesystem (`self.BPC_DamageSystem`))
  (add `/Game/Blueprints/DamageSystem/BPC_DamageSystem.OnDeath` _bpc_damagesystem (`|CreateDelegate` :!event `Death`))
  (add `/Game/Blueprints/DamageSystem/BPC_DamageSystem.OnDamageResponse` _bpc_damagesystem (`|CreateDelegate` :!event `HitResponse`)))