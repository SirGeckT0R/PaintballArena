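; Enemy character Blueprint with health, a floating health bar and movement and range data, likely for AI.
; Tick turns the health bar widget toward the player camera.
; Damage updates the bar and destroys the actor only when health would drop below zero.
; Helper functions expose attack and defend radii and a patrol route and map movement states to walk speeds, while weapon spawn-and-attach logic is disconnected.
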(event `self.ReceiveTick`
  (params (DeltaSeconds :type "Float (single-precision)"))
  (`self.RotateHealthBarToPlayer`))

(event `self.ReceiveBeginPlay`
  (bind _aswb_health_bar (cast `/Game/Blueprints/UI/WB_HealthBar` (`WidgetComponent.GetWidget` (`self.HealthBarWidget`))))
  (bind _output_get (set `self.HealthBar` _aswb_health_bar))
  (`/Game/Blueprints/UI/WB_HealthBar.SetHealth` _output_get (`self.Health`)))

(event `self.ReceiveAnyDamage`
  (params (Damage :type "Float (single-precision)") (DamageType :type "DamageType Object Reference") (InstigatedBy :type "Controller Object Reference") (DamageCauser :type "Actor Object Reference"))
  (bind _returnvalue (- (`self.Health`) Damage))
  (if (>= _returnvalue 0.0)
    (bind _output_get (set `self.Health` _returnvalue))
    (`/Game/Blueprints/UI/WB_HealthBar.SetHealth` (`self.HealthBar`) _output_get)
    (else
      (`self.Death`))))

(event `Death`
  ;[1 1 1] To cpp
  (`self.K2_DestroyActor`))

(fn `GetIdealRange`
  (returns (AttackRadius :type "Float (double-precision)") (DefendRadius :type "Float (double-precision)"))
  (return 150.0 550.0))

(fn `GetPatrolRoute`
  (returns (PatrolRoute :type "/Game/Blueprints/Enemies/AI/BP_PatrolRoute Object Reference"))
  (return (`self.PatrolRoute`)))

(fn `RotateHealthBarToPlayer`
  (bind _healthbarwidget (`self.HealthBarWidget`))
  (`SceneComponent.K2_SetWorldRotation` _healthbarwidget (`KismetMathLibrary.ComposeRotators` (`KismetMathLibrary.FindLookAtRotation` (`PlayerCameraManager.GetCameraLocation` (`GameplayStatics.GetPlayerCameraManager` 0)) (`SceneComponent.K2_GetComponentLocation` _healthbarwidget)) (struct :`Yaw` 180.0)) false false))

(fn `SetMovementSpeed`
  (params (MovementSpeed :type "/Game/Blueprints/Enemies/AI/Enums/E_MovementSpeed Enum" :default "NewEnumerator0"))
  (returns (SpeedValue :type "Float (double-precision)"))
  (bind _output_get (set `CharacterMovementComponent.MaxWalkSpeed` (select `/Game/Blueprints/Enemies/AI/Enums/E_MovementSpeed` MovementSpeed :`NewEnumerator1` 200.0 :`NewEnumerator2` 300.0 :`NewEnumerator3` 500.0 :!type "Float (single-precision)") (`self.CharacterMovement`)))
  (return _output_get))

(fn `UpdateHealthBar`
  (set `/Game/Blueprints/UI/WB_HealthBar.Health` (`self.Health`) (`self.HealthBar`))
  (return))

(fn `UserConstructionScript`)