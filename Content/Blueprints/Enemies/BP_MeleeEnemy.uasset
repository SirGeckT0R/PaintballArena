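; BP_MeleeEnemy is a melee enemy character that spawns and equips a weapon in its right-hand socket on BeginPlay.
; Attack plays a given montage, with notifies triggering a debug-drawn forward sphere trace that sends fixed damage to the hit actor.
; Montage completion or interruption signals attack end.
; Weapon equip and unequip fire callbacks, and SetMovementSpeed maps movement states to walk speeds.
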(event `self.ReceiveBeginPlay`
  (`parent.ReceiveBeginPlay`)
  (`/Game/Blueprints/Enemies/AI/BPI_EnemyAI.EquipWeapon`))

(event `/Game/Blueprints/Enemies/AI/BPI_EnemyAI.EquipWeapon`
  (`self.SpawnWeapon` (struct))
  (bind _returnvalue (`self.K2_AttachToComponent` (`self.Weapon`) (`self.Mesh`) "RightHandWeaponSocket" "KeepRelative" "KeepRelative" "KeepRelative" true))
  (set `self.IsWieldingWeapon` _returnvalue)
  (`self.OnWeaponEquipped`))

(event `/Game/Blueprints/Enemies/AI/BPI_EnemyAI.UnequipWeapon`
  (bind _weapon (`self.Weapon`))
  (`self.OnWeaponUnequiped`)
  (`self.K2_DetachFromActor` _weapon "KeepRelative" "KeepRelative" "KeepRelative")
  (`self.K2_DestroyActor` _weapon))

(event `/Game/Blueprints/Enemies/AI/BPI_EnemyAI.Attack`
  (params (MontageToPlay :type "AnimMontage Object Reference") (UseDefaultAttackMontage :type Boolean))
  (bind _returnvalue (`self.K2_GetActorLocation`))
  (bind _notifyname (`|PlayMontage` (`self.Mesh`) MontageToPlay)
    (:`OnCompleted`
      (`self.OnAttackEnd` :!label _label))
    (:`OnInterrupted`
      (goto _label))
    (:`OnNotifyBegin`
      (switch `name` _notifyname
        (:`Slash`
          (bind (_outhit _returnvalue_2) (`KismetSystemLibrary.SphereTraceSingleForObjects` :`Start` _returnvalue :`End` (+ _returnvalue (* (`self.GetActorForwardVector`) 150.0)) :`Radius` 40.0 :`ObjectTypes` (`|MakeArray` "ObjectTypeQuery7" "ObjectTypeQuery3" :!type "EObjectTypeQuery Enum") :`DrawDebugType` "ForDuration"))
          (if _returnvalue_2
            (message `/Game/Blueprints/DamageSystem/BPI_Damagable.TakeDamage` (`.HitActor` (`GameplayStatics.BreakHitResult` _outhit)) (make `/Game/Blueprints/DamageSystem/S_DamageInfo` 30.0 "NewEnumerator1") self)))))))

(fn `SetMovementSpeed`
  (params (MovementSpeed :type "/Game/Blueprints/Enemies/AI/Enums/E_MovementSpeed Enum" :default "NewEnumerator0"))
  (returns (SpeedValue :type "Float (double-precision)"))
  (set `CharacterMovementComponent.MaxWalkSpeed` (select `/Game/Blueprints/Enemies/AI/Enums/E_MovementSpeed` MovementSpeed :`NewEnumerator1` 200.0 :`NewEnumerator2` 300.0 :`NewEnumerator3` 800.0 :!type "Float (single-precision)") (`self.CharacterMovement`))
  (return 0.0))

(fn `UserConstructionScript`
  (`parent.UserConstructionScript`))