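; Ranged enemy character that spawns a hitscan weapon, attaches it to its right-hand socket and fires at its AI controller's attack target.
; Attack plays a montage whose notifies toggle crouching or trigger a pawn-only debug line trace from the weapon to the target, damaging the hit actor.
; The enemy is uninterruptible during the montage and signals attack end afterwards.
; It also supplies ideal combat ranges and movement speeds.
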(event `self.ReceiveBeginPlay`
  (`parent.ReceiveBeginPlay`)
  (`self.EquipWeapon`))

(event `self.Attack`
  (params (MontageToPlay :type "AnimMontage Object Reference") (UseDefaultAttackMontage :type Boolean))
  (bind (_attack_target _location) (`self.GetAttackTarget `))
  (bind _notifyname (`self.AttackMontage` (select `bool` (and UseDefaultAttackMontage (`KismetSystemLibrary.IsValid` (`self.DefaultAttackMontage`))) :`false` MontageToPlay :`true` (`self.DefaultAttackMontage`)))
    (:`then`
      (set `/Game/Blueprints/DamageSystem/BPC_DamageSystem.IsInterruptible` false (`self.BPC_DamageSystem`)))
    (:`OnCompleted`
      (`self.OnAttackEnd` :!label _label)
      (set `/Game/Blueprints/DamageSystem/BPC_DamageSystem.IsInterruptible` true (`self.BPC_DamageSystem`)))
    (:`OnInterrupted`
      (goto _label))
    (:`OnNotifyBegin`
      (switch `name` _notifyname
        (:`Fire`
          (bind (_outhit _returnvalue) (`KismetSystemLibrary.LineTraceSingleForObjects` :`Start` (`self.K2_GetActorLocation` (`self.WeaponActor`)) :`End` _location :`ObjectTypes` (`|MakeArray` "ObjectTypeQuery3" :!type "EObjectTypeQuery Enum") :`DrawDebugType` "ForDuration"))
          (if _returnvalue
            (message `/Game/Blueprints/DamageSystem/BPI_Damagable.TakeDamage` (`.HitActor` (`GameplayStatics.BreakHitResult` _outhit)) (make `/Game/Blueprints/DamageSystem/S_DamageInfo` 1.0 "NewEnumerator2" "NewEnumerator1") (`self.GetOwner`))
            (`KismetSystemLibrary.PrintString` "HitTarget")))
        (:`UnCrouch`
          (`self.ExitCrouchedState`))
        (:`Crouch`
          (`self.EnterCrouchedState`))))))

(event `self.EquipWeapon`
  (bind _returnvalue (`|SpawnActorFromClass` "/Game/Blueprints/Weapons/BP_HitScanWeapon.BP_HitScanWeapon_C" (`KismetMathLibrary.MakeTransform` (0.0 0.0 0.0)) "Undefined" "MultiplyWithRoot" null null))
  (bind _output_get (set `self.WeaponActor` _returnvalue))
  (bind _returnvalue_2 (`self.K2_AttachToComponent` _output_get (`self.Mesh`) "RightHandWeaponSocket" "KeepRelative" "KeepRelative" "KeepRelative" true))
  (set `self.IsWieldingWeapon` _returnvalue_2)
  (`self.OnWeaponEquipped`))

(fn `GetAttackTarget `
  (returns (`Attack Target` :type "Actor Object Reference") (Location :type "Vector Structure"))
  (locals (ActorLocation :type "Vector Structure"))
  (bind _asaic_enemy_base (cast `/Game/Blueprints/Enemies/AI/AIC_EnemyBase` (`AIBlueprintHelperLibrary.GetAIController` self)))
  (bind _attack_target (`/Game/Blueprints/Enemies/AI/AIC_EnemyBase.Attack Target` _asaic_enemy_base)
    (:`then`
      (bind (_returnvalue_x _returnvalue_y _returnvalue_z) (`KismetMathLibrary.BreakVector` (`self.K2_GetActorLocation` _attack_target)))
      (return _attack_target (`KismetMathLibrary.MakeVector` _returnvalue_x _returnvalue_y (+ _returnvalue_z 50.0))))
    (:`else`)))

(fn `GetIdealRange`
  (returns (AttackRadius :type "Float (double-precision)") (DefendRadius :type "Float (double-precision)"))
  (return 1800.0 1400.0))

(fn `GetPatrolRoute`
  (returns (PatrolRoute :type "/Game/Blueprints/Enemies/AI/BP_PatrolRoute Object Reference"))
  (return null))

(fn `SetMovementSpeed`
  (params (MovementSpeed :type "/Game/Blueprints/Enemies/AI/Enums/E_MovementSpeed Enum" :default "NewEnumerator0"))
  (returns (SpeedValue :type "Float (double-precision)"))
  (set `CharacterMovementComponent.MaxWalkSpeed` (select `/Game/Blueprints/Enemies/AI/Enums/E_MovementSpeed` MovementSpeed :`NewEnumerator1` 200.0 :`NewEnumerator2` 300.0 :`NewEnumerator3` 500.0 :!type "Float (single-precision)") (`self.CharacterMovement`))
  (return 0.0))

(fn `UserConstructionScript`
  (`parent.UserConstructionScript`))