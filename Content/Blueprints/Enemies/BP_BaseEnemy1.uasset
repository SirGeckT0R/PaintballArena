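; Base enemy character that pairs an AI controller with a damage component and a camera-facing health bar.
; Damage feeds the component, whose bound events play a hit montage before turning the AI on the attacker, or on death set it dead and drop an ammo pickup.
; It also supplies patrol route claiming, movement speeds and combat ranges to the AI.
; Attack and weapon equip are print-only placeholders.
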(event `self.ReceiveTick`
  (params (DeltaSeconds :type "Float (single-precision)"))
  (`self.RotateHealthBarToPlayer`))

(event `self.ReceiveBeginPlay`
  (`KismetSystemLibrary.Delay` 0.2)
  (bind _asaic_enemy_base (cast `/Game/Blueprints/Enemies/AI/AIC_EnemyBase` (`AIBlueprintHelperLibrary.GetAIController` self)))
  (set `self.AICEnemyBase` _asaic_enemy_base)
  (bind _aswb_health_bar (cast `/Game/Blueprints/UI/WB_HealthBar` (`WidgetComponent.GetWidget` (`self.HealthBarWidget`))))
  (set `self.HealthBar` _aswb_health_bar)
  (`self.UpdateHealthBar`))

(event `self.ReceiveAnyDamage`
  (params (Damage :type "Float (single-precision)") (DamageType :type "DamageType Object Reference") (InstigatedBy :type "Controller Object Reference") (DamageCauser :type "Actor Object Reference"))
  (`self.TakeDamage` (make `/Game/Blueprints/DamageSystem/S_DamageInfo` Damage "NewEnumerator2") DamageCauser)
  (`self.UpdateHealthBar`))

(event `/Game/Blueprints/Enemies/AI/BPI_EnemyAI.UnequipWeapon`
  (`KismetSystemLibrary.PrintString` "unequip weapon"))

(event `/Game/Blueprints/Enemies/AI/BPI_EnemyAI.EquipWeapon`
  (`KismetSystemLibrary.PrintString` "equip weapon"))

(event `Death`
  (`/Game/Blueprints/Enemies/AI/AIC_EnemyBase.SetStateAsDead` (`self.AICEnemyBase`))
  (`ActorComponent.K2_DestroyComponent` (`self.HealthBarWidget`))
  (message `/Game/Blueprints/Enemies/AI/BPI_EnemyAI.UnequipWeapon` self)
  (`/Game/Blueprints/Enemies/AI/AIC_EnemyBase.SetStateAsDead` (`self.AICEnemyBase`))
  (`|SpawnActorFromClass` "/Game/Blueprints/Weapons/BP_AmmoPickup.BP_AmmoPickup_C" (`self.GetTransform`) "AlwaysSpawn" "MultiplyWithRoot" null null))

(event `HitResponse`
  (params (DamageResponse :type "/Game/Blueprints/DamageSystem/E_DamageResponse Enum" :default "NewEnumerator0") (DamageCauser :type "Actor Object Reference"))
  (bind _aicenemybase (`self.AICEnemyBase`))
  (`MovementComponent.StopMovementImmediately` (`self.CharacterMovement`))
  (`/Game/Blueprints/Enemies/AI/AIC_EnemyBase.SetStateAsFrozen` (`self.AICEnemyBase`))
  (`|PlayMontage` (`self.Mesh`) (`self.HitReactionMontage`)
    (:`OnCompleted`
      _)
    (:`OnInterrupted`
      _))
  (`/Game/Blueprints/Enemies/AI/AIC_EnemyBase.SetStateAsAttacking` _aicenemybase DamageCauser true)
  (`/Game/Blueprints/Enemies/AI/AIC_EnemyBase.OnHostileDetected` _aicenemybase DamageCauser))

(event `/Game/Blueprints/Enemies/AI/BPI_EnemyAI.EnterCrouchedState`
  (`self.Crouch`))

(event `/Game/Blueprints/Enemies/AI/BPI_EnemyAI.ExitCrouchedState`
  (`self.UnCrouch`))

(event `/Game/Blueprints/Enemies/AI/BPI_EnemyAI.Attack`
  (params (MontageToPlay :type "AnimMontage Object Reference") (UseDefaultAttackMontage :type Boolean))
  (`KismetSystemLibrary.PrintString` "Here Supposed to be an attack"))

(event `/Game/Blueprints/Enemies/AI/BPI_EnemyAI.Find and Set Patrol Route`
  (bind _nearestroute (`/Game/Blueprints/Core/GM_ShooterProjectGameModeBase.GetNearestPatrolRouteToActor` (cast `/Game/Blueprints/Core/GM_ShooterProjectGameModeBase` (`GameplayStatics.GetGameMode`) :!pure true) self))
  (`/Engine/EditorBlueprintResources/StandardMacros.IsValid` _nearestroute
    (:`Is Valid`
      (bind _output_get (set `self.PatrolRoute` _nearestroute))
      (set `/Game/Blueprints/Enemies/AI/BP_PatrolRoute.IsTaken` true _output_get))))

(fn `GetCurrentHealth`
  (returns (CurrentHealth :type "Float (double-precision)"))
  (return (`/Game/Blueprints/DamageSystem/BPC_DamageSystem.Health` (`self.BPC_DamageSystem`))))

(fn `GetIdealRange`
  (returns (AttackRadius :type "Float (double-precision)") (DefendRadius :type "Float (double-precision)"))
  (return 150.0 550.0))

(fn `GetMaxHealth`
  (returns (MaxHealth :type "Float (double-precision)"))
  (return (`/Game/Blueprints/DamageSystem/BPC_DamageSystem.MaxHealth` (`self.BPC_DamageSystem`))))

(fn `GetPatrolRoute`
  (returns (PatrolRoute :type "/Game/Blueprints/Enemies/AI/BP_PatrolRoute Object Reference"))
  (return (`self.PatrolRoute`)))

(fn `Heal`
  (params (Amount :type "Float (double-precision)"))
  (returns (NewHealth :type "Float (double-precision)"))
  (bind _newhealth (`/Game/Blueprints/DamageSystem/BPC_DamageSystem.Heal` (`self.BPC_DamageSystem`) Amount))
  (`self.UpdateHealthBar`)
  (return _newhealth))

(fn `IsDead`
  (returns (IsDead :type Boolean))
  (return (`/Game/Blueprints/DamageSystem/BPC_DamageSystem.IsDead` (`self.BPC_DamageSystem`))))

(fn `ReleasePatrolRoute`
  (returns (IsSuccesfull :type Boolean))
  (set `/Game/Blueprints/Enemies/AI/BP_PatrolRoute.IsTaken` false (`self.PatrolRoute`))
  (return true))

(fn `RotateHealthBarToPlayer`
  (bind _healthbarwidget (`self.HealthBarWidget`))
  (`/Engine/EditorBlueprintResources/StandardMacros.IsValid` (`self.HealthBarWidget`)
    (:`Is Valid`
      (`SceneComponent.K2_SetWorldRotation` _healthbarwidget (`KismetMathLibrary.ComposeRotators` (`KismetMathLibrary.FindLookAtRotation` (`PlayerCameraManager.GetCameraLocation` (`GameplayStatics.GetPlayerCameraManager` 0)) (`SceneComponent.K2_GetComponentLocation` _healthbarwidget)) (struct :`Yaw` 180.0)) false false))))

(fn `SetMovementSpeed`
  (params (MovementSpeed :type "/Game/Blueprints/Enemies/AI/Enums/E_MovementSpeed Enum" :default "NewEnumerator0"))
  (returns (SpeedValue :type "Float (double-precision)"))
  (bind _output_get (set `CharacterMovementComponent.MaxWalkSpeed` (select `/Game/Blueprints/Enemies/AI/Enums/E_MovementSpeed` MovementSpeed :`NewEnumerator1` 200.0 :`NewEnumerator2` 300.0 :`NewEnumerator3` 500.0 :!type "Float (single-precision)") (`self.CharacterMovement`)))
  (return _output_get))

(fn `TakeDamage`
  (params (DamageInfo :type "/Game/Blueprints/DamageSystem/S_DamageInfo Structure") (`DamageCauser ` :type "Actor Object Reference"))
  (returns (WasDamaged :type Boolean))
  (bind _wasdamaged (`/Game/Blueprints/DamageSystem/BPC_DamageSystem.TakeDamage` (`self.BPC_DamageSystem`) DamageInfo `DamageCauser `))
  (`self.UpdateHealthBar`)
  (return _wasdamaged))

(fn `UpdateHealthBar`
  (bind _currenthealth (`self.GetCurrentHealth`))
  (`/Game/Blueprints/UI/WB_HealthBar.SetHealth` (`self.HealthBar`) _currenthealth)
  (return))

(fn `UserConstructionScript`
  (bind _bpc_damagesystem (`self.BPC_DamageSystem`))
  (add `/Game/Blueprints/DamageSystem/BPC_DamageSystem.OnDeath` _bpc_damagesystem (`|CreateDelegate` :!event `Death`))
  (add `/Game/Blueprints/DamageSystem/BPC_DamageSystem.OnDamageResponse` _bpc_damagesystem (`|CreateDelegate` :!event `HitResponse`)))