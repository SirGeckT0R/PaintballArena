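; Base enemy character that pairs an AI controller with a damage component and an overhead health bar kept turned toward the player camera.
; Damage and healing pass through BPC_DamageSystem and refresh the bar.
; Hit response freezes the AI for a montage, then targets the damage causer, while death ragdolls, stops AI logic and destroys the actor.
; Getters expose ranges, patrol route and speed presets; attack and weapon equip events are print-only placeholders.
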(event `self.ReceiveTick`
  (params (DeltaSeconds :type "Float (single-precision)"))
  (`self.RotateHealthBarToPlayer`))

(event `self.ReceiveBeginPlay`
  (`KismetSystemLibrary.Delay` 0.2)
  (bind _asaic_enemy_base (cast `/Game/Blueprints/Enemies/AI/AIC_EnemyBase` (`AIBlueprintHelperLibrary.GetAIController` self)))
  (set `self.AICEnemyBase` _asaic_enemy_base)
  (bind _aswb_health_bar (cast `/Game/Blueprints/UI/WB_HealthBar` (`WidgetComponent.GetWidget` (`self.HealthBarWidget`))))
  (set `self.HealthBar` _aswb_health_bar)
  (`self.UpdateHealthBar`))

(event `self.ReceiveAnyDamage`
  (params (Damage :type "Float (single-precision)") (DamageType :type "DamageType Object Reference") (InstigatedBy :type "Controller Object Reference") (DamageCauser :type "Actor Object Reference"))
  (`self.TakeDamage` (make `/Game/Blueprints/DamageSystem/S_DamageInfo` Damage "NewEnumerator2") DamageCauser)
  (`self.UpdateHealthBar`))

(event `/Game/Blueprints/Enemies/AI/BPI_EnemyAI.UnequipWeapon`
  (`KismetSystemLibrary.PrintString` "unequip weapon"))

(event `/Game/Blueprints/Enemies/AI/BPI_EnemyAI.EquipWeapon`
  (`KismetSystemLibrary.PrintString` "equip weapon"))

(event `Death`
  (bind _aicenemybase (`self.AICEnemyBase`))
  (bind _mesh (`self.Mesh`))
  (`KismetSystemLibrary.PrintString` "Enemy Dead")
  (`PrimitiveComponent.SetSimulatePhysics` _mesh true)
  (`PrimitiveComponent.SetCollisionEnabled` _mesh "QueryAndPhysics")
  (`BrainComponent.StopLogic` (`AIController.BrainComponent` _aicenemybase) "Death")
  (`/Game/Blueprints/Enemies/AI/AIC_EnemyBase.SetStateAsDead` _aicenemybase)
  (`KismetSystemLibrary.Delay` 5.0)
  (`self.K2_DestroyActor`))

(event `HitResponse`
  (params (DamageResponse :type "/Game/Blueprints/DamageSystem/E_DamageResponse Enum" :default "NewEnumerator0") (DamageCauser :type "Actor Object Reference"))
  (`MovementComponent.StopMovementImmediately` (`self.CharacterMovement`))
  (`/Game/Blueprints/Enemies/AI/AIC_EnemyBase.SetStateAsFrozen` (`self.AICEnemyBase`))
  (`|PlayMontage` (`self.Mesh`) (`self.HitReactionMontage`)
    (:`OnCompleted`
      _)
    (:`OnInterrupted`
      _))
  (`/Game/Blueprints/Enemies/AI/AIC_EnemyBase.SetStateAsAttacking` (`self.AICEnemyBase`) DamageCauser true))

(event `/Game/Blueprints/Enemies/AI/BPI_EnemyAI.EnterCrouchedState`
  (`self.Crouch`))

(event `/Game/Blueprints/Enemies/AI/BPI_EnemyAI.ExitCrouchedState`
  (`self.UnCrouch`))

(event `/Game/Blueprints/Enemies/AI/BPI_EnemyAI.Attack`
  (params (MontageToPlay :type "AnimMontage Object Reference") (UseDefaultAttackMontage :type Boolean))
  (`KismetSystemLibrary.PrintString` "Here Supposed to be an attack"))

(fn `GetCurrentHealth`
  (returns (CurrentHealth :type "Float (double-precision)"))
  (return (`/Game/Blueprints/DamageSystem/BPC_DamageSystem.Health` (`self.BPC_DamageSystem`))))

(fn `GetIdealRange`
  (returns (AttackRadius :type "Float (double-precision)") (DefendRadius :type "Float (double-precision)"))
  (return 150.0 550.0))

(fn `GetMaxHealth`
  (returns (MaxHealth :type "Float (double-precision)"))
  (return (`/Game/Blueprints/DamageSystem/BPC_DamageSystem.MaxHealth` (`self.BPC_DamageSystem`))))

(fn `GetPatrolRoute`
  (returns (PatrolRoute :type "/Game/Blueprints/Enemies/AI/BP_PatrolRoute Object Reference"))
  (return (`self.PatrolRoute`)))

(fn `Heal`
  (params (Amount :type "Float (double-precision)"))
  (returns (NewHealth :type "Float (double-precision)"))
  (bind _newhealth (`/Game/Blueprints/DamageSystem/BPC_DamageSystem.Heal` (`self.BPC_DamageSystem`) Amount))
  (`self.UpdateHealthBar`)
  (return _newhealth))

(fn `IsDead`
  (returns (IsDead :type Boolean))
  (return (`/Game/Blueprints/DamageSystem/BPC_DamageSystem.IsDead` (`self.BPC_DamageSystem`))))

(fn `RotateHealthBarToPlayer`
  (bind _healthbarwidget (`self.HealthBarWidget`))
  (`SceneComponent.K2_SetWorldRotation` _healthbarwidget (`KismetMathLibrary.ComposeRotators` (`KismetMathLibrary.FindLookAtRotation` (`PlayerCameraManager.GetCameraLocation` (`GameplayStatics.GetPlayerCameraManager` 0)) (`SceneComponent.K2_GetComponentLocation` _healthbarwidget)) (struct :`Yaw` 180.0)) false false))

(fn `SetMovementSpeed`
  (params (MovementSpeed :type "/Game/Blueprints/Enemies/AI/Enums/E_MovementSpeed Enum" :default "NewEnumerator0"))
  (returns (SpeedValue :type "Float (double-precision)"))
  (bind _output_get (set `CharacterMovementComponent.MaxWalkSpeed` (select `/Game/Blueprints/Enemies/AI/Enums/E_MovementSpeed` MovementSpeed :`NewEnumerator1` 200.0 :`NewEnumerator2` 300.0 :`NewEnumerator3` 500.0 :!type "Float (single-precision)") (`self.CharacterMovement`)))
  (return _output_get))

(fn `TakeDamage`
  (params (DamageInfo :type "/Game/Blueprints/DamageSystem/S_DamageInfo Structure") (`DamageCauser ` :type "Actor Object Reference"))
  (returns (WasDamaged :type Boolean))
  (bind _wasdamaged (`/Game/Blueprints/DamageSystem/BPC_DamageSystem.TakeDamage` (`self.BPC_DamageSystem`) DamageInfo `DamageCauser `))
  (`self.UpdateHealthBar`)
  (return _wasdamaged))

(fn `UpdateHealthBar`
  (bind _currenthealth (`self.GetCurrentHealth`))
  (`/Game/Blueprints/UI/WB_HealthBar.SetHealth` (`self.HealthBar`) _currenthealth)
  (return))

(fn `UserConstructionScript`
  (bind _bpc_damagesystem (`self.BPC_DamageSystem`))
  (add `/Game/Blueprints/DamageSystem/BPC_DamageSystem.OnDeath` _bpc_damagesystem (`|CreateDelegate` :!event `Death`))
  (add `/Game/Blueprints/DamageSystem/BPC_DamageSystem.OnDamageResponse` _bpc_damagesystem (`|CreateDelegate` :!event `HitResponse`)))