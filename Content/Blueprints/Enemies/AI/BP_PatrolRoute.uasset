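; BP_PatrolRoute is an enemy AI patrol route that uses the points of a PatrolRoute spline as waypoints.
; IncrementPatrolPoint steps CurrentIndex by Direction and reverses it at the first and last points, so the route runs back and forth instead of looping.
; GetSplinePointAsWorldPosition returns the world location of the spline point at the current index.
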(event `IncrementPatrolPoint`
  (bind _output_get (set `self.CurrentIndex` (+ (`self.CurrentIndex`) (`self.Direction`))))
  (if (== _output_get (- (`SplineComponent.GetNumberOfSplinePoints` (`self.PatrolRoute`)) 1))
    (set `self.Direction` -1)
    (elif (== (`self.CurrentIndex`) 0)
      (set `self.Direction` 1))))

(fn `GetSplinePointAsWorldPosition`
  (returns (Location :type "Vector Structure"))
  (return (`SplineComponent.GetLocationAtSplinePoint` (`self.PatrolRoute`) (`self.CurrentIndex`) "World")))

(fn `UserConstructionScript`)