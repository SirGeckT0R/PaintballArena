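; Melee enemy Blueprint that extends a parent enemy class, equipping a weapon on BeginPlay and implementing a montage-driven Attack event.
; Attack plays either the supplied montage or, when requested and valid, the default one.
; Montage notifies run a forward sphere trace, with debug drawing, that sends melee damage to the hit actor through a TakeDamage message.
; Completion or interruption of the montage calls OnAttackEnd.
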(event `self.ReceiveBeginPlay`
  (`parent.ReceiveBeginPlay`)
  (`EnemyAI.EquipWeapon`))

(event `self.ReceiveTick`
  (params (DeltaSeconds :type "Float (single-precision)"))
  (`parent.ReceiveTick` 0.0))

(event `self.Attack`
  (params (MontageToPlay :type "AnimMontage Object Reference") (UseDefaultAttackMontage :type Boolean))
  (bind _returnvalue (`self.K2_GetActorLocation`))
  (bind _notifyname (`|PlayMontage` (`self.Mesh`) (select `bool` (and UseDefaultAttackMontage (`KismetSystemLibrary.IsValid` (`self.DefaultAttackMontage`))) :`false` MontageToPlay :`true` (`self.DefaultAttackMontage`)))
    (:`OnCompleted`
      (`self.OnAttackEnd` :!label _label))
    (:`OnInterrupted`
      (goto _label))
    (:`OnNotifyBegin`
      (switch `name` _notifyname
        (:`Slash`
          (bind (_outhit _returnvalue_2) (`KismetSystemLibrary.SphereTraceSingleForObjects` :`Start` _returnvalue :`End` (+ _returnvalue (* (`self.GetActorForwardVector`) 150.0)) :`Radius` 40.0 :`ObjectTypes` (`|MakeArray` "ObjectTypeQuery7" "ObjectTypeQuery3" :!type "EObjectTypeQuery Enum") :`DrawDebugType` "ForDuration"))
          (if _returnvalue_2
            (message `Damagable.TakeDamage` (`.HitActor` (`GameplayStatics.BreakHitResult` _outhit)) (make `SDamageInfo` 30.0) self)))))))

(fn `UserConstructionScript`
  (`parent.UserConstructionScript`))