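; Ranged enemy character that equips a weapon on BeginPlay and attacks the AI controller's target with a hitscan rifle.
; Attack plays a montage whose notifies fire the shot or toggle crouching, and blocks interruption until it ends.
; Shots line-trace from the rifle toward a raised point on the target, trigger weapon effects and send damage through TakeDamageMessage.
; It also supplies ideal combat ranges and maps movement states to walk speeds.
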(event `self.Attack`
  (params (MontageToPlay :type "AnimMontage Object Reference") (UseDefaultAttackMontage :type Boolean))
  (bind _asrifle (cast `Rifle` (`self.Weapon`)))
  (bind (_attack_target _currentlocation) (`self.GetAttackTarget `))
  (bind _notifyname (`self.AttackMontage` MontageToPlay)
    (:`then`
      (set `/Game/Blueprints/DamageSystem/BPC_DamageSystem.IsInterruptible` false (`self.BPC_DamageSystem`)))
    (:`OnCompleted`
      (`self.OnAttackEnd` :!label _label)
      (set `/Game/Blueprints/DamageSystem/BPC_DamageSystem.IsInterruptible` true (`self.BPC_DamageSystem`)))
    (:`OnInterrupted`
      (goto _label))
    (:`OnNotifyBegin`
      (switch `name` _notifyname
        (:`Fire`
          (bind _returnvalue (`self.K2_GetActorLocation` _asrifle))
          (bind (_outhit _returnvalue_2) (`KismetSystemLibrary.LineTraceSingleForObjects` _returnvalue (+ _returnvalue (* (`KismetMathLibrary.Normal` (`KismetMathLibrary.GreaterGreater_VectorRotator` (`KismetMathLibrary.MakeVector` 1.0) (`KismetMathLibrary.FindLookAtRotation` (`self.K2_GetActorLocation` _asrifle) _currentlocation))) (`self.ShotDistance`))) (`|MakeArray` "ObjectTypeQuery7" "ObjectTypeQuery3" :!type "EObjectTypeQuery Enum")))
          (`Weapon.AttackEffects` _asrifle _outhit)
          (if _returnvalue_2
            (message `/Game/Blueprints/DamageSystem/BPI_Damagable.TakeDamage` (`.HitActor` (`GameplayStatics.BreakHitResult` _outhit)) (make `/Game/Blueprints/DamageSystem/S_DamageInfo` (`self.Damage`) "NewEnumerator2" "NewEnumerator1") (`self.GetOwner`))
            (`KismetSystemLibrary.PrintString` "HitTarget")))
        (:`UnCrouch`
          (`EnemyAI.ExitCrouchedState`))
        (:`Crouch`
          (`EnemyAI.EnterCrouchedState`))))))

(event `self.ReceiveBeginPlay`
  (`parent.ReceiveBeginPlay`)
  (`EnemyAI.EquipWeapon`))

(fn `GetAttackTarget `
  (returns (`Attack Target` :type "Actor Object Reference") (CurrentLocation :type "Vector Structure"))
  (locals (ActorLocation :type "Vector Structure"))
  (bind _asaic_enemy_base (cast `/Game/Blueprints/Enemies/AI/AIC_EnemyBase` (`AIBlueprintHelperLibrary.GetAIController` self)))
  (bind _attack_target (`/Game/Blueprints/Enemies/AI/AIC_EnemyBase.Attack Target` _asaic_enemy_base)
    (:`then`
      (bind (_returnvalue_x _returnvalue_y _returnvalue_z) (`KismetMathLibrary.BreakVector` (`self.K2_GetActorLocation` _attack_target)))
      (return _attack_target (`KismetMathLibrary.MakeVector` _returnvalue_x _returnvalue_y (+ _returnvalue_z 50.0))))
    (:`else`)))

(fn `GetIdealRange`
  (returns (AttackRadius :type "Float (single-precision)") (DefendRadius :type "Float (single-precision)"))
  (return 1800.0 1600.0))

(fn `SetMovementSpeed`
  (params (Speed :type "E_MovementSpeed Enum" :default "Idle"))
  (returns (ReturnValue :type "Float (single-precision)"))
  (set `CharacterMovementComponent.MaxWalkSpeed` (select `E_MovementSpeed` Speed :`Walking` 200.0 :`Jogging` 300.0 :`Running` 500.0 :!type "Float (single-precision)") (`self.CharacterMovement`))
  (return 0.0))

(fn `UserConstructionScript`
  (`parent.UserConstructionScript`))