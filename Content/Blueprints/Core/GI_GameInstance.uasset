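; Game Instance that holds the Master, SFX and Music volume levels and applies them to the game's audio.
; OnAudioVolumeChange overrides the sound class volume in the mix matching the audio type, pushes a mix modifier, then stores the value through ChangeVolumeByType.
; InitVolume reapplies all three stored volumes in one loop, using the array index to select each mix and class pair.
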(event `OnAudioVolumeChange`
  (params (Value :type "Float (double-precision)") (TypeOfAudio :type "/Game/Blueprints/Core/E_TypesOfAudio Enum" :default "NewEnumerator1"))
  (`GameplayStatics.SetSoundMixClassOverride` (select `/Game/Blueprints/Core/E_TypesOfAudio` TypeOfAudio :`NewEnumerator0` "/Game/Aesthetics/Audio/SoundMixes/SCM_MasterMix.SCM_MasterMix" :`NewEnumerator2` "/Game/Aesthetics/Audio/SoundMixes/SCM_SFXMix.SCM_SFXMix" :`NewEnumerator3` "/Game/Aesthetics/Audio/SoundMixes/SCM_MusicMix.SCM_MusicMix" :!type "SoundMix Object Reference") (select `/Game/Blueprints/Core/E_TypesOfAudio` TypeOfAudio :`NewEnumerator0` "/Game/Aesthetics/Audio/SoundClasses/SC_Master.SC_Master" :`NewEnumerator2` "/Game/Aesthetics/Audio/SoundClasses/SC_SFX.SC_SFX" :`NewEnumerator3` "/Game/Aesthetics/Audio/SoundClasses/SC_Music.SC_Music" :!type "SoundClass Object Reference") Value 1.0 0.0)
  (`GameplayStatics.PushSoundMixModifier` null)
  (`self.ChangeVolumeByType` TypeOfAudio Value))

(fn `ChangeVolumeByType`
  (params (Selection :type "/Game/Blueprints/Core/E_TypesOfAudio Enum" :default "NewEnumerator1") (Value :type "Float (double-precision)"))
  (switch `/Game/Blueprints/Core/E_TypesOfAudio` Selection
    (:`NewEnumerator0`
      (set `self.MasterVolume` Value))
    (:`NewEnumerator2`
      (set `self.SFXVolume` Value))
    (:`NewEnumerator3`
      (set `self.MusicVolume` Value))))

(fn `InitVolume`
  (for (_array_element _array_index) (`|MakeArray` (`self.MasterVolume`) (`self.SFXVolume`) (`self.MusicVolume`) :!type "Float (single-precision)")
    (`GameplayStatics.SetSoundMixClassOverride` (select `int` _array_index :`0` "/Game/Aesthetics/Audio/SoundMixes/SCM_MasterMix.SCM_MasterMix" :`1` "/Game/Aesthetics/Audio/SoundMixes/SCM_SFXMix.SCM_SFXMix" :`2` "/Game/Aesthetics/Audio/SoundMixes/SCM_MusicMix.SCM_MusicMix" :!type "SoundMix Object Reference") (select `int` _array_index :`0` "/Game/Aesthetics/Audio/SoundClasses/SC_Master.SC_Master" :`1` "/Game/Aesthetics/Audio/SoundClasses/SC_SFX.SC_SFX" :`2` "/Game/Aesthetics/Audio/SoundClasses/SC_Music.SC_Music" :!type "SoundClass Object Reference") _array_element 1.0 0.0)
    (`GameplayStatics.PushSoundMixModifier` null)))